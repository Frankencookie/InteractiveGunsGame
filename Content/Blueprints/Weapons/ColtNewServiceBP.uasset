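; Colt New Service revolver weapon with animated, clickable trigger, cylinder release, ejector and bullet slots.
; Firing cocks via timeline if needed, advancing the six-slot cylinder, then drops the hammer and fires the magazine's next bullet as a raycast with flash, sound and camera shake.
; CylinderMagazine tracks rounds and handles ejector and bullet clicks, while a material parameter marks spent rounds.
; Timelines swing the cylinder open or closed, auto-closing when manipulate mode ends.
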(event OnClicked(Ejector)
  (params (TouchedComponent :type Primitive%20Component%20Object%20Reference) (ButtonPressed :type Key%20Structure :default "None"))
  (bind _cylindermagazine (Variables|Default|GetCylinderMagazine))
  ;[0.15 0.15 0.15 0.5] Opening/Closing cylinder
  ;;[0.15 0.15 0.15 0.5] Ejector
  (if (Variables|/Script/InteractiveGuns.MagazineComponentBase|GetMagazineRemoved _cylindermagazine)
    (Class|CylinderMagazineComponent|HandleEjectorClicked _cylindermagazine)))

(event OnClicked(CylinderRelease)
  (params (TouchedComponent :type Primitive%20Component%20Object%20Reference) (ButtonPressed :type Key%20Structure :default "None"))
  ;[0.15 0.15 0.15 0.5] Opening/Closing cylinder
  ;;[0.15 0.15 0.15 0.5] Cylinder release is clicked
  (if (Variables|/Script/InteractiveGuns.MagazineComponentBase|GetMagazineRemoved (Variables|Default|GetCylinderMagazine))
    (Utilities|FlowControl|Sequence
      (:then_0
        ;;[0.15 0.15 0.15 0.5] Open Cylinder
        (bind _rotatecylindercam (Timeline|OpenCylinder Stop)
          (:Update
            (Transformation|SetRelativeRotation (Variables|Default|GetEjector) (Math|Rotator|MakeRotator _rotatecylindercam 0.0 0.0) false false))))
      (:then_1
        ;;[0.15 0.15 0.15 0.5] Close Cylinder
        (Variables|/Script/InteractiveGuns.MagazineComponentBase|SetMagazineRemoved (Variables|Default|GetCylinderMagazine) false)
        (bind _output_get (Variables|Default|SetCylinderClosingStartRotation (.roll (Variables|/Script/Engine.SceneComponent|GetRelativeRotation (Variables|Default|GetEjector)))))
        (bind _normalisedprogress (Timeline|CloseCylinder PlayFromStart)
          (:Update
            (Transformation|SetRelativeRotation (Variables|Default|GetEjector) (Math|Rotator|MakeRotator (Math|Float|Lerp _output_get 0.0 _normalisedprogress) 0.0 0.0) false false)))))
    (else
      (Variables|/Script/InteractiveGuns.MagazineComponentBase|SetMagazineRemoved (Variables|Default|GetCylinderMagazine) true)
      (Timeline|OpenCylinder PlayFromStart))))

(event OnClicked(Trigger)
  (params (TouchedComponent :type Primitive%20Component%20Object%20Reference) (ButtonPressed :type Key%20Structure :default "None"))
  (bind _cylindermagazine (Variables|Default|GetCylinderMagazine))
  (bind _hammer (Variables|Default|GetHammer))
  (bind _muzzlepos (Variables|Default|GetMuzzlePos))
  (bind _returnvalue (Transformation|GetWorldLocation _muzzlepos))
  ;[0.15 0.15 0.15 0.5] Player pulls trigger
  (bind _returnvalue_2 (CallFunction|CanFire))
  (if _returnvalue_2
    (Variables|Default|SetTryingToFire true)
    (if (Variables|Default|GetCocked)
      ;[0.15 0.15 0.15 0.5] Reset hammer and trigger positions
      (Audio|PlaySoundatLocation "/Game/Audio/gunHammerStrike.gunHammerStrike" (Transformation|GetWorldLocation _hammer) "0, 0, 0" 1.0 1.0 0.0 0 0 0 0 :!label _label)
      (Transformation|SetRelativeRotation (Variables|Default|GetTrigger) "0, 0, 0" false false)
      (Transformation|SetRelativeRotation _hammer "0, 0, 0" false false)
      ;[0.15 0.15 0.15 0.5] Stop here if magazine removed
      (if (Variables|/Script/InteractiveGuns.MagazineComponentBase|GetMagazineRemoved _cylindermagazine)
        (Variables|Default|SetTryingToFire false :!label _label_2)
        (else
          ;[0.15 0.15 0.15 0.5] Get next bullet and try to fire it
          (bind _returnvalue_3 (Class|MagazineComponentBase|GetNextBullet _cylindermagazine))
          (if (Utilities|IsValid _returnvalue_3)
            (bind _returnvalue_4 (Class|Bullet|TryFire _returnvalue_3))
            (if _returnvalue_4
              (CallFunction|UpdateBulletMaterials (Variables|/Script/InteractiveGuns.CylinderMagazineComponent|GetIndex _cylindermagazine) true)
              ;[0.7031 0.1318 0.1318 0.5] Fire
              (Class|WeaponBase|ShootRaycast (Math|Vector|GetForwardVector _muzzlepos) 1e+04)
              (Camera|PlayWorldCameraShake "/Game/Blueprints/GunshotCameraShake.GunshotCameraShake_C" _returnvalue 0.0 1e+02)
              (Class|WeaponBase|HandleonWeaponFired)
              (Audio|PlaySoundatLocation "/Game/Audio/Gunshot1_Cue.Gunshot1_Cue" _returnvalue "0, 0, 0" 1.0 1.0 0.0 0 0 0 0)
              (bind _flash (Timeline|MuzzleFlash PlayFromStart)
                (:Update
                  (Rendering|Components|Light|SetIntensity (Variables|Default|GetPointLight) (Math|Float|Lerp 0.0 (Variables|Default|GetMuzzleFlashPeakBrightness) _flash))
                  (Variables|Default|SetTryingToFire false)))
              (else
                (goto _label_2))))))
      (else
        ;[0.15 0.15 0.15 0.5] Cock and strike
        (Variables|Default|SetCylinderStartRotation (.roll (Variables|/Script/Engine.SceneComponent|GetRelativeRotation (Variables|Default|GetCylinder))))
        (bind _value (Timeline|Cock PlayFromStart)
          (:Update
            (Transformation|SetRelativeRotation (Variables|Default|GetHammer) (Math|Rotator|MakeRotator 0.0 (Math|Float|Lerp 0.0 3e+01 _value) 0.0) false false)
            (Transformation|SetRelativeRotation (Variables|Default|GetCylinder) (Math|Rotator|MakeRotator (Math|Float|Lerp (Variables|Default|GetCylinderStartRotation) (+ (Variables|Default|GetCylinderStartRotation) 6e+01) _value) 0.0 0.0) false false)
            (Transformation|SetRelativeRotation (Variables|Default|GetTrigger) (Math|Rotator|MakeRotator 0.0 (Math|Float|Lerp 0.0 -3e+01 _value) 0.0) false false))
          (:Finished
            (Class|CylinderMagazineComponent|IncrementCylinderIndex _cylindermagazine)
            (goto _label)))))))

(event Custom|OnBulletClicked_Event
  (params (index :type Integer))
  ;[0.15 0.15 0.15 0.5] Handle Bullet clicking
  (Class|CylinderMagazineComponent|HandleBulletClicked (Variables|Default|GetCylinderMagazine) index)
  (Rendering|Material|SetScalarParameterValueonMaterials (Utilities|Array|Get(acopy) (Variables|/Script/InteractiveGuns.MagazineComponentBase|GetbulletSlots (Variables|Default|GetCylinderMagazine)) index) "Fired" 0.0))

(event EventBeginPlay
  ;[0.15 0.15 0.15 0.5] Bind clicking bullets
  (for _array_element (Variables|/Script/InteractiveGuns.MagazineComponentBase|GetbulletSlots (Variables|Default|GetCylinderMagazine))
    (EventDispatchers|AssignOnBulletClicked _array_element (delegate Custom|OnBulletClicked_Event))))

(event EventManipulateModeEnd
  ;[0.15 0.15 0.15 0.5] Opening/Closing cylinder
  ;;[0.15 0.15 0.15 0.5] Close cylinder if open when manipulate mode ends
  (if (Variables|/Script/InteractiveGuns.MagazineComponentBase|GetMagazineRemoved (Variables|Default|GetCylinderMagazine))
    (Utilities|FlowControl|Sequence
      (:then_0
        ;;[0.15 0.15 0.15 0.5] Open Cylinder
        (bind _rotatecylindercam (Timeline|OpenCylinder Stop)
          (:Update
            (Transformation|SetRelativeRotation (Variables|Default|GetEjector) (Math|Rotator|MakeRotator _rotatecylindercam 0.0 0.0) false false))))
      (:then_1
        ;;[0.15 0.15 0.15 0.5] Close Cylinder
        (Variables|/Script/InteractiveGuns.MagazineComponentBase|SetMagazineRemoved (Variables|Default|GetCylinderMagazine) false)
        (bind _output_get (Variables|Default|SetCylinderClosingStartRotation (.roll (Variables|/Script/Engine.SceneComponent|GetRelativeRotation (Variables|Default|GetEjector)))))
        (bind _normalisedprogress (Timeline|CloseCylinder PlayFromStart)
          (:Update
            (Transformation|SetRelativeRotation (Variables|Default|GetEjector) (Math|Rotator|MakeRotator (Math|Float|Lerp _output_get 0.0 _normalisedprogress) 0.0 0.0) false false)))))))

(event EventPrimaryAttack
  (bind _cylindermagazine (Variables|Default|GetCylinderMagazine))
  (bind _hammer (Variables|Default|GetHammer))
  (bind _muzzlepos (Variables|Default|GetMuzzlePos))
  (bind _returnvalue (Transformation|GetWorldLocation _muzzlepos))
  ;[0.15 0.15 0.15 0.5] Player pulls trigger
  (bind _returnvalue_2 (CallFunction|CanFire))
  (if _returnvalue_2
    (Variables|Default|SetTryingToFire true)
    (if (Variables|Default|GetCocked)
      ;[0.15 0.15 0.15 0.5] Reset hammer and trigger positions
      (Audio|PlaySoundatLocation "/Game/Audio/gunHammerStrike.gunHammerStrike" (Transformation|GetWorldLocation _hammer) "0, 0, 0" 1.0 1.0 0.0 0 0 0 0 :!label _label)
      (Transformation|SetRelativeRotation (Variables|Default|GetTrigger) "0, 0, 0" false false)
      (Transformation|SetRelativeRotation _hammer "0, 0, 0" false false)
      ;[0.15 0.15 0.15 0.5] Stop here if magazine removed
      (if (Variables|/Script/InteractiveGuns.MagazineComponentBase|GetMagazineRemoved _cylindermagazine)
        (Variables|Default|SetTryingToFire false :!label _label_2)
        (else
          ;[0.15 0.15 0.15 0.5] Get next bullet and try to fire it
          (bind _returnvalue_3 (Class|MagazineComponentBase|GetNextBullet _cylindermagazine))
          (if (Utilities|IsValid _returnvalue_3)
            (bind _returnvalue_4 (Class|Bullet|TryFire _returnvalue_3))
            (if _returnvalue_4
              (CallFunction|UpdateBulletMaterials (Variables|/Script/InteractiveGuns.CylinderMagazineComponent|GetIndex _cylindermagazine) true)
              ;[0.7031 0.1318 0.1318 0.5] Fire
              (Class|WeaponBase|ShootRaycast (Math|Vector|GetForwardVector _muzzlepos) 1e+04)
              (Camera|PlayWorldCameraShake "/Game/Blueprints/GunshotCameraShake.GunshotCameraShake_C" _returnvalue 0.0 1e+02)
              (Class|WeaponBase|HandleonWeaponFired)
              (Audio|PlaySoundatLocation "/Game/Audio/Gunshot1_Cue.Gunshot1_Cue" _returnvalue "0, 0, 0" 1.0 1.0 0.0 0 0 0 0)
              (bind _flash (Timeline|MuzzleFlash PlayFromStart)
                (:Update
                  (Rendering|Components|Light|SetIntensity (Variables|Default|GetPointLight) (Math|Float|Lerp 0.0 (Variables|Default|GetMuzzleFlashPeakBrightness) _flash))
                  (Variables|Default|SetTryingToFire false)))
              (else
                (goto _label_2))))))
      (else
        ;[0.15 0.15 0.15 0.5] Cock and strike
        (Variables|Default|SetCylinderStartRotation (.roll (Variables|/Script/Engine.SceneComponent|GetRelativeRotation (Variables|Default|GetCylinder))))
        (bind _value (Timeline|Cock PlayFromStart)
          (:Update
            (Transformation|SetRelativeRotation (Variables|Default|GetHammer) (Math|Rotator|MakeRotator 0.0 (Math|Float|Lerp 0.0 3e+01 _value) 0.0) false false)
            (Transformation|SetRelativeRotation (Variables|Default|GetCylinder) (Math|Rotator|MakeRotator (Math|Float|Lerp (Variables|Default|GetCylinderStartRotation) (+ (Variables|Default|GetCylinderStartRotation) 6e+01) _value) 0.0 0.0) false false)
            (Transformation|SetRelativeRotation (Variables|Default|GetTrigger) (Math|Rotator|MakeRotator 0.0 (Math|Float|Lerp 0.0 -3e+01 _value) 0.0) false false))
          (:Finished
            (Class|CylinderMagazineComponent|IncrementCylinderIndex _cylindermagazine)
            (goto _label)))))))

(fn ConstructionScript
  ;[0.15 0.15 0.15 0.5] This feels like shit
  (for _index (range 0 5)
    (Utilities|Array|Add (Variables|/Script/InteractiveGuns.MagazineComponentBase|GetbulletSlots (Variables|Default|GetCylinderMagazine)) (Utilities|Select :Index _index :Option%200 (Variables|Default|GetBullet0) :Option%201 (Variables|Default|GetBullet1) :Option%202 (Variables|Default|GetBullet2) :Option%203 (Variables|Default|GetBullet3) :Option%204 (Variables|Default|GetBullet4) :Option%205 (Variables|Default|GetBullet5)))))

(fn CanFire
  (return (not (Variables|Default|GetTryingToFire))))

(fn UpdateBulletMaterials
  (params (Index :type Integer) (Fired :type Boolean))
  (Rendering|Material|SetScalarParameterValueonMaterials (Utilities|Array|Get(acopy) (Variables|/Script/InteractiveGuns.MagazineComponentBase|GetbulletSlots (Variables|Default|GetCylinderMagazine)) Index) "Fired" (Math|Conversions|ToFloat(Boolean) Fired)))